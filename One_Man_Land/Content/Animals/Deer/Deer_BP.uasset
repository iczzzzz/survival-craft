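; Deer animal character that wanders the navmesh, flees from the player or vehicles, and can be killed and skinned for items.
; Recursive AI MoveTo loops drive roaming and fleeing to random reachable points, with a Sight overlap toggling between them and setting speed and DeerAnimBP flags.
; Hit drains Live until Die swaps in DeadMesh.
; Skin spawns PickUpGives items into the player's inventory and destroys the deer.
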(event OnComponentBeginOverlap(Sight)
  (params (OverlappedComponent :type Primitive%20Component%20Object%20Reference) (OtherActor :type Actor%20Object%20Reference) (OtherComp :type Primitive%20Component%20Object%20Reference) (OtherBodyIndex :type Integer) (bFromSweep :type Boolean) (SweepResult :type Hit%20Result%20Structure%20%28by%20ref%29))
  ;[1 1 1] Sight Detection
  (Utilities|Casting|CastToFirstPersonCharacter OtherActor
    (:then
      _)
    (:CastFailed
      (Utilities|Casting|CastToWheeledVehicle OtherActor)))
  (Variables|Default|SetPlayerNoticed true)
  (Variables|/Script/Engine.CharacterMovementComponent|SetMaxWalkSpeed (Variables|Character|GetCharacterMovement) 5e+04)
  (bind _asdeer_anim_bp (Utilities|Casting|CastToDeerAnimBP (Components|SkeletalMesh|GetAnimInstance (Variables|Character|GetMesh))))
  (Variables|/Game/Animals/Deer/DeerAnimBP.DeerAnimBP_C|SetCanRun _asdeer_anim_bp true)
  (Variables|/Game/Animals/Deer/DeerAnimBP.DeerAnimBP_C|SetCanWalk _asdeer_anim_bp false)
  (CallFunction|RunAway))

(event OnComponentEndOverlap(Sight)
  (params (OverlappedComponent :type Primitive%20Component%20Object%20Reference) (OtherActor :type Actor%20Object%20Reference) (OtherComp :type Primitive%20Component%20Object%20Reference) (OtherBodyIndex :type Integer))
  ;[1 1 1] Sight Detection
  (Utilities|Casting|CastToFirstPersonCharacter OtherActor
    (:then
      _)
    (:CastFailed
      (Utilities|Casting|CastToWheeledVehicle OtherActor)))
  (Variables|Default|SetPlayerNoticed false)
  (bind _asdeer_anim_bp (Utilities|Casting|CastToDeerAnimBP (Components|SkeletalMesh|GetAnimInstance (Variables|Character|GetMesh))))
  (Variables|/Game/Animals/Deer/DeerAnimBP.DeerAnimBP_C|SetCanWalk _asdeer_anim_bp true)
  (Variables|/Game/Animals/Deer/DeerAnimBP.DeerAnimBP_C|SetCanRun _asdeer_anim_bp false)
  (Variables|/Script/Engine.CharacterMovementComponent|SetMaxWalkSpeed (Variables|Character|GetCharacterMovement) 1e+02)
  (CallFunction|Roam))

(event Custom|Roam
  (bind _mesh (Variables|Character|GetMesh))
  (bind _charactermovement (Variables|Character|GetCharacterMovement))
  (bind _returnvalue (Components|SkeletalMesh|GetAnimInstance _mesh))
  ;[1 1 1] Roam
  (AI|AIMoveTo self (.RandomLocation (Class|NavigationSystemV1|GetRandomPointinNavigableRadius (Transformation|GetActorLocation) 1.5e+03 0 0)) 0 5.0 false
    (:OnSuccess
      (if (Variables|Default|GetPlayerNoticed)
        (bind _asdeer_anim_bp (Utilities|Casting|CastToDeerAnimBP _returnvalue))
        (Variables|/Game/Animals/Deer/DeerAnimBP.DeerAnimBP_C|SetCanWalk _asdeer_anim_bp false)
        (Variables|/Game/Animals/Deer/DeerAnimBP.DeerAnimBP_C|SetCanRun _asdeer_anim_bp true)
        (Variables|/Script/Engine.CharacterMovementComponent|SetMaxWalkSpeed _charactermovement 5e+03)
        (CallFunction|RunAway)
        (else
          (bind _asdeer_anim_bp_2 (Utilities|Casting|CastToDeerAnimBP _returnvalue))
          (Variables|/Game/Animals/Deer/DeerAnimBP.DeerAnimBP_C|SetCanWalk _asdeer_anim_bp_2 false)
          (Variables|/Script/Engine.CharacterMovementComponent|SetMaxWalkSpeed _charactermovement 0.0)
          (Utilities|FlowControl|Delay 3.0)
          (Variables|/Script/Engine.CharacterMovementComponent|SetMaxWalkSpeed _charactermovement 1e+02)
          (Variables|/Game/Animals/Deer/DeerAnimBP.DeerAnimBP_C|SetCanWalk _asdeer_anim_bp_2 true)
          (CallFunction|Roam))))
    (:OnFail
      (CallFunction|Roam))))

(event Custom|Run%20Away
  (bind _charactermovement (Variables|Character|GetCharacterMovement))
  ;[1 1 1] Run Away
  (AI|AIMoveTo self (.RandomLocation (Class|NavigationSystemV1|GetRandomPointinNavigableRadius (Transformation|GetActorLocation) 3e+03 0 0)) 0 5.0 false
    (:OnSuccess
      (if (and (Variables|Default|GetPlayerNoticed) (> 2.5e+03 (Transformation|GetDistanceTo (Variables|Default|GetCharacterRef))))
        (Variables|/Script/Engine.CharacterMovementComponent|SetMaxWalkSpeed _charactermovement 5e+03)
        (CallFunction|RunAway)
        (else
          (Variables|/Script/Engine.CharacterMovementComponent|SetMaxWalkSpeed _charactermovement 1e+02)
          (CallFunction|Roam))))
    (:OnFail
      (CallFunction|RunAway))))

(event EventBeginPlay
  (bind _deadmesh (Variables|Default|GetDeadMesh))
  ;[1 1 1] Begin
  (bind _asfirst_person_character (Utilities|Casting|CastToFirstPersonCharacter (Game|GetPlayerCharacter 0)))
  (Variables|Default|SetCharacterRef _asfirst_person_character)
  (Rendering|SetVisibility _deadmesh false false)
  (Collision|SetCollisionEnabled _deadmesh "NoCollision")
  (bind _asdeer_anim_bp (Utilities|Casting|CastToDeerAnimBP (Components|SkeletalMesh|GetAnimInstance (Variables|Character|GetMesh))))
  (Variables|/Game/Animals/Deer/DeerAnimBP.DeerAnimBP_C|SetCanWalk _asdeer_anim_bp true)
  (CallFunction|Roam))

(fn ConstructionScript)

(fn Hit
  (params (Damage :type Float%20%28single-precision%29))
  (if (not (Variables|Default|GetisDead))
    (bind _output_get (Variables|Default|Set?Live (Math|Float|Max(Float) (- (Variables|Default|Get?Live) Damage) 0.0)))
    (if (== _output_get 0.0)
      (CallFunction|Die))))

(fn Die
  (bind _mesh (Variables|Character|GetMesh))
  (bind _deadmesh (Variables|Default|GetDeadMesh))
  (Variables|Default|SetisDead true)
  (Pawn|Components|CharacterMovement|DisableMovement (Variables|Character|GetCharacterMovement))
  (Rendering|SetVisibility _mesh false false)
  (Collision|SetCollisionEnabled _mesh "NoCollision")
  (Rendering|SetVisibility _deadmesh true false)
  (Collision|SetCollisionEnabled _deadmesh "QueryAndPhysics"))

(fn Skin
  (for _array_element (Variables|Default|GetPickUpGives)
    (bind _returnvalue (Game|SpawnActorfromClass _array_element (Math|Transform|MakeTransform "0, 0, 0") "Undefined" 0 0))
    (Default|AddtoInventory (Variables|Default|GetCharacterRef) _returnvalue))
  (Actor|DestroyActor))